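; Speaker actor made of clickable parts: cabinet, woofers, horn tweeter, feet, accent plate, and a cover frame with screen.
; Clicks forward to an injected speaker logic reference as accent, speaker or cabinet events, while screen clicks only print a message.
; Initialization stores that reference and shows or hides the cover per CoverActive, loosening its collision when hidden.
; Getter functions expose the meshes by part group.
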(event `self.Foot_FL.OnClicked`
  (params (TouchedComponent :type "PrimitiveComponent Object Reference") (ButtonPressed :type "Key Structure"))
  ;[1 1 1] Accent Clicked
  (`/Game/Spkrs/BP/SpeakerLogic_BP.AccentClicked` (`self.Speaker_Logic_Reference`) :!label _label))

(event `self.Foot_FR.OnClicked`
  (params (TouchedComponent :type "PrimitiveComponent Object Reference") (ButtonPressed :type "Key Structure"))
  ;[1 1 1] Accent Clicked
  (goto _label))

(event `self.Frame.OnClicked`
  (params (TouchedComponent :type "PrimitiveComponent Object Reference") (ButtonPressed :type "Key Structure"))
  ;[1 1 1] Accent Clicked
  (goto _label))

(event `self.Foot_BL.OnClicked`
  (params (TouchedComponent :type "PrimitiveComponent Object Reference") (ButtonPressed :type "Key Structure"))
  ;[1 1 1] Accent Clicked
  (goto _label))

(event `self.Foot_BR.OnClicked`
  (params (TouchedComponent :type "PrimitiveComponent Object Reference") (ButtonPressed :type "Key Structure"))
  ;[1 1 1] Accent Clicked
  (goto _label))

(event `self.AccentPlate.OnClicked`
  (params (TouchedComponent :type "PrimitiveComponent Object Reference") (ButtonPressed :type "Key Structure"))
  ;[1 1 1] Accent Clicked
  (goto _label))

(event `self.Woofers.OnClicked`
  (params (TouchedComponent :type "PrimitiveComponent Object Reference") (ButtonPressed :type "Key Structure"))
  ;[1 1 1] Speakers Clicked
  (`/Game/Spkrs/BP/SpeakerLogic_BP.SpeakerClicked` (`self.Speaker_Logic_Reference`) :!label _label_2))

(event `self.HornTweeter.OnClicked`
  (params (TouchedComponent :type "PrimitiveComponent Object Reference") (ButtonPressed :type "Key Structure"))
  ;[1 1 1] Speakers Clicked
  (goto _label_2))

(event `self.Screen.OnClicked`
  (params (TouchedComponent :type "PrimitiveComponent Object Reference") (ButtonPressed :type "Key Structure"))
  ;[1 1 1] Screen Clicked
  (`KismetSystemLibrary.PrintString` "Screen Clicked"))

(event `self.Cabinette.OnClicked`
  (params (TouchedComponent :type "PrimitiveComponent Object Reference") (ButtonPressed :type "Key Structure"))
  ;[1 1 1] Cabinet Clicked
  (`/Game/Spkrs/BP/SpeakerLogic_BP.CabinetClicked` (`self.Speaker_Logic_Reference`)))

(fn `GetAccentComponents`
  (returns (FootMeshes :type "Array of MeshComponent Object Reference") (AccentMeshes :type "Array of MeshComponent Object Reference"))
  (return (`|MakeArray` (`self.Foot_BR`) (`self.Foot_FL`) (`self.Foot_FR`) (`self.Foot_BL`)) (`|MakeArray` (`self.AccentPlate`) (`self.Frame`))))

(fn `GetCabinetComponent`
  (returns (CabinetMesh :type "MeshComponent Object Reference"))
  ;[1 1 1] CabinetMeshを戻り値として返す
  (return (`self.Cabinette`)))

(fn `GetScreenComponent`
  (returns (NewParam :type "MeshComponent Object Reference"))
  (return (`self.Screen`)))

(fn `GetSpeakerComponents`
  (returns (TweeterMesh :type "MeshComponent Object Reference") (WooferMesh :type "MeshComponent Object Reference"))
  (return (`self.HornTweeter`) (`self.Woofers`)))

(fn `InitializeSpeakerBP`
  (params (SpeakerLogicBP :type "/Game/Spkrs/BP/SpeakerLogic_BP Object Reference"))
  (`|ExecutionSequence`
    (:`then_0`
      (set `self.Speaker_Logic_Reference` SpeakerLogicBP))
    (:`then_1`
      ;[1 1 1] CheckCoverActice
      (if (`self.Cover Active`)
        ;;[0.0368 1 0] True
        (`SceneComponent.SetVisibility` (`self.Frame`) true false)
        (`SceneComponent.SetVisibility` (`self.Screen`) true false)
        (else
          ;;[1 0.04724 0] False
          (`SceneComponent.SetVisibility` (`self.Frame`) false false)
          (`SceneComponent.SetVisibility` (`self.Screen`) false false)
          (`PrimitiveComponent.SetCollisionResponseToChannel` (`self.Frame`) "ECC_WorldStatic" "ECR_Ignore")
          (`PrimitiveComponent.SetCollisionResponseToAllChannels` (`self.Screen`) "ECR_Ignore"))))))

(fn `UserConstructionScript`)